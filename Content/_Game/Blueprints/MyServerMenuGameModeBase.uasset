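; Server menu game mode that tracks connected players and pushes the player list to each client's menu controller.
; InitNewPlayer parses the PlayerName connection option into BP_MyPlayerState, then triggers a broadcast, as does Logout.
; The broadcast builds player infos from the GameState PlayerArray, with placeholder level and ready values, and sends them through each ServerMenuPC_BP.
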(event Custom|SendConnectedClients
  (for _array_element (Variables|/Script/Engine.GameStateBase|GetPlayerArray (Game|GetGameState))
    (bind _asserver_menu_pc_bp (Utilities|Casting|CastToServerMenuPC_BP (Components|GetOwner _array_element)))
    (bind _playerinfos (CallFunction|CreateConnectedPlayerInfos))
    (Default|TriggerUpdatePlayerListfromServer _asserver_menu_pc_bp _playerinfos)))

(event EventBeginPlay)

(event EventTick
  (params (DeltaSeconds :type Float%20%28single-precision%29)))

(event EventLogout
  (params (Exiting :type Controller%20Object%20Reference))
  (CallFunction|SendConnectedClients))

(fn ConstructionScript)

(fn InitNewPlayer
  (params (NewPlayerController :type Player%20Controller%20Object%20Reference) (UniqueId :type Unique%20Net%20Id%20Repl%20Structure%20%28by%20ref%29) (Options :type String) (Portal :type String))
  (bind _asbp_my_player_state (Utilities|Casting|CastToBP_MyPlayerState (Variables|/Script/Engine.Controller|GetPlayerState NewPlayerController)))
  (Default|SetPlayerUsername _asbp_my_player_state (Class|GameplayStatics|ParseOption Options "PlayerName"))
  (CallFunction|SendConnectedClients))

(fn CreateConnectedPlayerInfos
  (for _array_element (Variables|/Script/Engine.GameStateBase|GetPlayerArray (Game|GetGameState))
    (bind _asserver_menu_pc_bp (Utilities|Casting|CastToServerMenuPC_BP (Components|GetOwner _array_element)))
    (bind _asbp_my_player_state (Utilities|Casting|CastToBP_MyPlayerState (Variables|/Script/Engine.Controller|GetPlayerState _asserver_menu_pc_bp)))
    (Utilities|Array|Add (LocalVariables|GetPlayerInfosLocal) (Utilities|Struct|MakeF_PlayerInfo (Variables|/Game/_Game/Blueprints/BP_MyPlayerState.BP_MyPlayerState_C|GetPlayerUserName _asbp_my_player_state) 0 false)))
  (return (LocalVariables|GetPlayerInfosLocal)))